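; AI controller for the farm game's turret that runs its behavior tree and tracks enemies through AI perception.
; Sensing an Enemy-tagged actor cancels the turret's timer, writes the actor to the Blackboard Target and turns the turret's meshes red.
; Losing sight passes an event to the turret's Forget, apparently a delayed callback to OnForgetTarget, which clears Target and restores white.
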(event `self.ReceiveBeginPlay`
  (`self.RunBehaviorTree` "/Game/_Farmer/AI/Turret/BT_Turret.BT_Turret"))

(event `self.AIPerception.OnTargetPerceptionUpdated`
  (params (Actor :type "Actor Object Reference") (Stimulus :type "AIStimulus Structure"))
  (`self.ElaboratePerception` Actor Stimulus))

(event `OnForgetTarget`
  (`BlackboardComponent.SetValueAsObject` (`AIBlueprintHelperLibrary.GetBlackboard` null) "Target" null)
  (`self.ChangeColor` "/Game/_Farmer/Materials/MI_White.MI_White"))

(fn `ChangeColor`
  (params (Material :type "MaterialInterface Object Reference"))
  (for _array_element (`self.K2_GetComponentsByClass` (`self.K2_GetPawn`) "/Script/Engine.StaticMeshComponent")
    (`PrimitiveComponent.SetMaterial` _array_element 0 (`local.Material`))))

(fn `ElaboratePerception`
  (params (Actor :type "Actor Object Reference") (AIStimulus :type "AIStimulus Structure (by ref)"))
  (if (`self.ActorHasTag` (`local.Actor`) "Enemy")
    (bind _asbp_turret (cast `/Game/_Farmer/Blueprint/Turret/BP_Turret` (`self.K2_GetPawn`)))
    (`/Game/_Farmer/Blueprint/Turret/BP_Turret.ClearTimer` _asbp_turret)
    (if (`.bSuccessfullySensed` (break `AIStimulus` (`local.AIStimulus`)))
      (`BlackboardComponent.SetValueAsObject` (`AIBlueprintHelperLibrary.GetBlackboard` null) "Target" (`local.Actor`))
      (`self.ChangeColor` "/Game/_Farmer/Materials/MI_Red.MI_Red")
      (else
        (`/Game/_Farmer/Blueprint/Turret/BP_Turret.Forget` _asbp_turret (`|CreateDelegate` :!event `OnForgetTarget`))))))

(fn `UserConstructionScript`)