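; BP_FruitCollector is an interactable drop-off point where farmers deliver fruit, keeping a running count.
; When a BP_Farmer carrying fruit interacts, it clears the farmer's HasFruit flag, mirrors that to the farmer's AI Blackboard, and increments FruitsCollected.
; Tick prints the collected total on screen under a fixed key as a debug readout.
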(event `self.ReceiveTick`
  (params (DeltaSeconds :type "Float (single-precision)"))
  (`KismetSystemLibrary.PrintString` (`KismetStringLibrary.Concat_StrStr` "Collected fruits: " (`KismetStringLibrary.Conv_IntToString` (`self.FruitsCollected`))) true true (struct :`G` 0.66 :`B` 1.0 :`A` 1.0) 2.0 "999"))

(event `self.Interact`
  (params (Interacter :type "Actor Object Reference"))
  (bind _asbp_farmer (cast `/Game/_Farmer/Blueprint/BP_Farmer` Interacter))
  (if (`/Game/_Farmer/Blueprint/BP_Farmer.HasFruit` _asbp_farmer)
    (`KismetSystemLibrary.PrintString` "Fruit collected")
    (set `/Game/_Farmer/Blueprint/BP_Farmer.HasFruit` false _asbp_farmer)
    (`BlackboardComponent.SetValueAsBool` (`AIBlueprintHelperLibrary.GetBlackboard` _asbp_farmer) "HasFruit" false)
    (`/Engine/EditorBlueprintResources/StandardMacros.IncrementInt` (`self.FruitsCollected`))))

(fn `UserConstructionScript`)