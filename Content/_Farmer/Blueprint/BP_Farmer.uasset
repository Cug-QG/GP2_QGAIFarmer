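; BP_Farmer is the farmer actor, able to interact with nearby objects and change its look.
; Interact runs a multi sphere trace on the Visibility channel around its own location, with one-frame debug drawing.
; Each hit actor implementing IInteractable receives an interact message with the farmer as argument.
; ChangeColor applies a supplied material to the mesh's first two material slots.
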(fn `ChangeColor`
  (params (Material :type "MaterialInterface Object Reference"))
  (`PrimitiveComponent.SetMaterial` (`self.Mesh`) 0 Material)
  (`PrimitiveComponent.SetMaterial` (`self.Mesh`) 1 Material))

(fn `Interact`
  (bind _returnvalue (`self.K2_GetActorLocation`))
  (bind _outhits (`KismetSystemLibrary.SphereTraceMulti` :`Start` _returnvalue :`End` _returnvalue :`Radius` 150.0 :`TraceChannel` "TraceTypeQuery1" :`DrawDebugType` "ForOneFrame"))
  (for _array_element _outhits
    (bind (_bblockinghit _binitialoverlap _time _distance _location _impactpoint _normal _impactnormal _physmat _hitactor) (`GameplayStatics.BreakHitResult` _array_element))
    (if (`KismetSystemLibrary.DoesImplementInterface` _hitactor "/Game/_Farmer/Blueprint/IInteractable.IInteractable_C")
      (message `/Game/_Farmer/Blueprint/IInteractable.Interact` _hitactor self))))

(fn `UserConstructionScript`)