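; BP_Field is a farm plot that a BP_Farmer plants and harvests through its Interact event.
; An empty plot consumes the farmer's seed, spawns a plant at its location and binds PlantGrown to the plant's grown delegate.
; Interacting once grown destroys the plant, resets the plot and gives the farmer fruit.
; Seed and fruit changes are written to both the farmer's variables and its Blackboard.
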(event `/Game/_Farmer/Blueprint/IInteractable.Interact`
  (params (Interacter :type "Actor Object Reference"))
  (bind _farmer (`self.Farmer`))
  (bind _farmer_2 (`self.Farmer`))
  (bind _asbp_farmer (cast `/Game/_Farmer/Blueprint/BP_Farmer` Interacter))
  (set `self.Farmer` _asbp_farmer)
  (if (`self.Planted`)
    (if (`self.Grown`)
      (set `self.Grown` false)
      (set `self.Planted` false)
      (`self.K2_DestroyActor` (`self.PlantInstance`))
      (`BlackboardComponent.SetValueAsBool` (`AIBlueprintHelperLibrary.GetBlackboard` _farmer_2) "HasFruit" true)
      (set `/Game/_Farmer/Blueprint/BP_Farmer.HasFruit` true _farmer_2))
    (elif (`/Game/_Farmer/Blueprint/BP_Farmer.HasSeed` (`self.Farmer`))
      (set `/Game/_Farmer/Blueprint/BP_Farmer.HasSeed` false _farmer)
      (`BlackboardComponent.SetValueAsBool` (`AIBlueprintHelperLibrary.GetBlackboard` _farmer) "HasSeed" false)
      (bind _returnvalue (`|SpawnActorFromClass` (`self.Plant`) (`KismetMathLibrary.MakeTransform` (`self.K2_GetActorLocation`)) "Undefined" "MultiplyWithRoot" null null))
      (bind _asbp_plant (cast `/Game/_Farmer/Blueprint/BP_Plant` _returnvalue))
      (bind _output_get (set `self.PlantInstance` _asbp_plant))
      (add `/Game/_Farmer/Blueprint/BP_Plant.GrownDelegate` _output_get (delegate `PlantGrown`))
      (set `self.Planted` true))))

(event `PlantGrown`
  (set `self.Grown` true))

(fn `UserConstructionScript`)